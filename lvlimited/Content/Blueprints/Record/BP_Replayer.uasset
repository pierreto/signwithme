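; Replays recorded two-hand gestures on left and right skeletal meshes in front of the camera.
; Pressing P stops playback or loads recordings from a save slot and calls Play, which captures the camera transform.
; Tick consumes frames as their timestamps pass, setting current pose snapshots and moving the enlarged meshes relative to that camera's location and yaw.
; Initial hand poses are saved at BeginPlay, and each hand can be hidden.
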(event `self.ReceiveBeginPlay`
  ;[1 1 1] Save initial hand pose
  (`SkeletalMeshComponent.SnapshotPose` (`self.SkeletalMeshL`) (`self.InitialLeftPose`))
  (`SkeletalMeshComponent.SnapshotPose` (`self.SkeletalMeshR`) (`self.InitialRightPose`))
  (`SceneComponent.SetVisibility` (`self.SkeletalMeshR`) (`self.ShowRight`) false)
  (`SceneComponent.SetVisibility` (`self.SkeletalMeshL`) (`self.ShowLeft`) false))

(event `self.ReceiveTick`
  (params (DeltaSeconds :type "Float (single-precision)"))
  (bind _recordings (`self.Recordings`))
  ;[1 1 1] Play recording
  (if (`self.IsPlayingRecording`)
    (`self.PlayRecording` _recordings DeltaSeconds)
    (if (or (<= (`KismetArrayLibrary.Array_Length` _recordings) 0) (>= (`self.CurrentReplayTime`) (`self.EndTime`)))
      (set `self.IsPlayingRecording` false))))

(event `Key|P`
  (params (Key :type "Key Structure"))
  ;[1 1 1] Load gesture recording and start playing
  (:`Released`
    (if (`self.IsPlayingRecording`)
      (set `self.IsPlayingRecording` false)
      (else
        (bind (_recordings _success) (`self.LoadRecording` (`self.SaveSlot`)))
        (if _success
          (`self.Play` _recordings)
          (else
            (`KismetSystemLibrary.PrintString` "Failed to load recording!" true true (struct :`R` 1.0 :`A` 1.0))))))))

(fn `GetWorldTransform`
  (params (Transform :type "Transform Structure"))
  (returns (WorldTransform :type "Transform Structure"))
  (bind _initialcameratransform (`self.InitialCameraTransform`))
  ;[1 1 1] Replay in front of camera
  (return (`KismetMathLibrary.MakeTransform` (+ (`KismetMathLibrary.RotateAngleAxis` (.location Transform) (.yaw (.rotation _initialcameratransform)) (0.0 0.0 1.0)) (.location _initialcameratransform)) (`KismetMathLibrary.MakeRotator` (.roll (.rotation Transform)) (.pitch (.rotation Transform)) (+ (.yaw (.rotation Transform)) (.yaw (.rotation _initialcameratransform)))) (5.0 5.0 5.0))))

(fn `HasOwnership`
  (returns (IsOwner :type Boolean))
  (return (== (`self.GetController`) (`GameplayStatics.GetPlayerController` 0))))

(fn `HideLeft`
  (`SceneComponent.SetVisibility` (`self.SkeletalMeshL`) false false)
  (set `self.ShowLeft` false))

(fn `HideRight`
  (`SceneComponent.SetVisibility` (`self.SkeletalMeshR`) false false)
  (set `self.ShowRight` false))

(fn `LoadRecording`
  (params (SaveSlot :type String))
  (returns (Recordings :type "Array of /Game/Blueprints/Record/GestureRecording Structure") (Success :type Boolean))
  (locals (Loaded :type Boolean) (LoadedRecordings :type "Array of /Game/Blueprints/Record/GestureRecording Structure"))
  (`GameplayStatics.CreateSaveGameObject` null)
  (bind _returnvalue (`GameplayStatics.LoadGameFromSlot` SaveSlot))
  (if (`KismetSystemLibrary.IsValid` _returnvalue)
    (bind _asrecording_save_game (cast `/Game/Blueprints/Record/RecordingSaveGame` _returnvalue))
    (set `local.LoadedRecordings` (`/Game/Blueprints/Record/RecordingSaveGame.Recordings` _asrecording_save_game))
    (set `local.Loaded` true))
  (return (`local.LoadedRecordings`) (`local.Loaded`)))

(fn `Play`
  (params (Recordings :type "Array of /Game/Blueprints/Record/GestureRecording Structure"))
  (set `self.IsPlayingRecording` true)
  (set `self.Recordings` Recordings)
  (set `self.CurrentReplayTime` 0.0)
  (set `self.InitialCameraTransform` (`SceneComponent.K2_GetComponentToWorld` (`self.Camera`))))

(fn `PlayRecording`
  (params (Recordings :type "Array of /Game/Blueprints/Record/GestureRecording Structure (by ref)") (DeltaTime :type "Float (double-precision)"))
  (bind (_leftpose _rightpose _lefttransform _righttransform _recordtime) (break `/Game/Blueprints/Record/GestureRecording` (`|GetArrayItem` Recordings)))
  (bind _output_get (set `self.CurrentReplayTime` (+ DeltaTime (`self.CurrentReplayTime`))))
  (if (>= _output_get _recordtime)
    (bind _worldtransform (`self.GetWorldTransform` _lefttransform))
    (`SceneComponent.K2_SetWorldTransform` (`self.SkeletalMeshL`) _worldtransform false false)
    (bind _worldtransform_2 (`self.GetWorldTransform` _righttransform))
    (`SceneComponent.K2_SetWorldTransform` (`self.SkeletalMeshR`) _worldtransform_2 false false)
    (set `self.CurrentLeftPose` _leftpose)
    (set `self.CurrentRightPose` _rightpose)
    (`KismetArrayLibrary.Array_Remove` Recordings)))

(fn `ResetHands`
  (set `self.CurrentLeftPose` (`self.InitialLeftPose`))
  (set `self.CurrentRightPose` (`self.InitialRightPose`)))

(fn `Stop`
  (set `self.IsPlayingRecording` false)
  (set `self.CurrentReplayTime` 0.0))

(fn `UserConstructionScript`)