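; VR recorder that captures two-hand gestures and saves them to save-game slots.
; While recording, each tick stores both hand mesh pose snapshots, transforms offset by camera location and yaw, and elapsed time.
; R toggles recording and saves on stop to a fixed slot; S saves snapshots to numbered slots.
; A position-based toggle is stubbed out, with its detection logic unconnected.
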(event `self.ReceiveBeginPlay`
  ;[1 1 1] Set tracking origin
  (`HeadMountedDisplayFunctionLibrary.SetTrackingOrigin` "Floor"))

(event `self.ReceiveTick`
  (params (DeltaSeconds :type "Float (single-precision)"))
  ;[1 1 1] Record gesture
  (`|ExecutionSequence`
    (:`then_0`
      (`self.SwitchToggle`
        (:`On`
          (`self.ToggleRecording`))))
    (:`then_1`
      (if (`self.IsRecording`)
        (`self.Record` DeltaSeconds)))))

(event `Key|S`
  (params (Key :type "Key Structure"))
  ;[1 1 1] Record a single frame
  (:`Released`
    (`self.Snapshot`)))

(event `Key|R`
  (params (Key :type "Key Structure"))
  ;[1 1 1] Start and stop recording from keyboard
  (:`Released`
    (`self.ToggleRecording`)))

(event `InputAction|Exit`
  (params (Key :type "Key Structure"))
  ;[1 1 1] Quit
  (:`Pressed`
    (`KismetSystemLibrary.QuitGame` null "Quit")))

(fn `DetectRecordingPostion`)

(fn `GetRelativeTransform`
  (params (Component :type "SceneComponent Object Reference"))
  (returns (Transform :type "Transform Structure"))
  (bind _returnvalue (`SceneComponent.K2_GetComponentToWorld` Component))
  (bind _returnvalue_2 (`SceneComponent.K2_GetComponentToWorld` (`self.Camera`)))
  (return (`KismetMathLibrary.MakeTransform` (- (.location _returnvalue) (.location _returnvalue_2)) (`KismetMathLibrary.MakeRotator` (.roll (.rotation _returnvalue)) (.pitch (.rotation _returnvalue)) (- (.yaw (.rotation _returnvalue)) (.yaw (.rotation _returnvalue_2)))) (.scale _returnvalue))))

(fn `Record`
  (params (DeltaSeconds :type "Float (double-precision)"))
  (locals (Delta :type "Float (double-precision)") (LeftPose :type "PoseSnapshot Structure") (RightPose :type "PoseSnapshot Structure"))
  (bind _leftpose (`local.LeftPose`))
  (bind _rightpose (`local.RightPose`))
  (bind _output_get (set `local.Delta` DeltaSeconds))
  (set `self.CurrentRecordTime` (+ _output_get (`self.CurrentRecordTime`)))
  (`KismetSystemLibrary.DrawDebugSphere` (`SceneComponent.K2_GetComponentLocation` (`self.SkeletalMeshR`)) 10.0 12 (struct :`R` 1.0 :`A` 1.0) -1.0)
  (`KismetSystemLibrary.DrawDebugSphere` (`SceneComponent.K2_GetComponentLocation` (`self.SkeletalMeshL`)) 10.0 12 (struct :`R` 1.0 :`A` 1.0) -1.0)
  (`SkeletalMeshComponent.SnapshotPose` (`self.SkeletalMeshL`) _leftpose)
  (`SkeletalMeshComponent.SnapshotPose` (`self.SkeletalMeshR`) _rightpose)
  (`KismetArrayLibrary.Array_Add` (`self.Recordings`) (make `/Game/Blueprints/Record/GestureRecording` _leftpose _rightpose (`self.GetRelativeTransform` (`self.SkeletalMeshL`)) (`self.GetRelativeTransform` (`self.SkeletalMeshR`)) (`self.CurrentRecordTime`))))

(fn `SaveRecording`
  (params (Recording :type "Array of /Game/Blueprints/Record/GestureRecording Structure") (SaveName :type String :default "TestSaveSlot"))
  (locals (Data :type "Array of String"))
  (`KismetSystemLibrary.PrintString` "Saving...")
  (bind _returnvalue (`GameplayStatics.CreateSaveGameObject` "/Game/Blueprints/Record/RecordingSaveGame.RecordingSaveGame_C"))
  (bind _output_get (set `/Game/Blueprints/Record/RecordingSaveGame.Recordings` Recording _returnvalue))
  (bind _returnvalue_2 (`GameplayStatics.SaveGameToSlot` _returnvalue SaveName (`/Game/Blueprints/Record/RecordingSaveGame.UserIndex` _returnvalue)))
  (if _returnvalue_2
    (`KismetSystemLibrary.PrintString` (`KismetStringLibrary.Concat_StrStr` "Saved " (`KismetStringLibrary.Conv_IntToString` (`KismetArrayLibrary.Array_Length` _output_get)) " recordings!"))))

(fn `Snapshot`
  (locals (LeftPose :type "PoseSnapshot Structure") (RightPose :type "PoseSnapshot Structure") (Recording :type "Array of /Game/Blueprints/Record/GestureRecording Structure"))
  (`SkeletalMeshComponent.SnapshotPose` (`self.SkeletalMeshL`) (`local.LeftPose`))
  (`SkeletalMeshComponent.SnapshotPose` (`self.SkeletalMeshR`) (`local.RightPose`))
  (`KismetArrayLibrary.Array_Add` (`local.Recording`) (make `/Game/Blueprints/Record/GestureRecording` (`local.LeftPose`) (`local.RightPose`) (`self.GetRelativeTransform` (`self.SkeletalMeshL`)) (`self.GetRelativeTransform` (`self.SkeletalMeshR`)) (`self.CurrentRecordTime`)))
  (`self.SaveRecording` (`local.Recording`) (`KismetStringLibrary.Concat_StrStr` "TestSaveSlot" (`KismetStringLibrary.Conv_IntToString` (`self.Snapcount`))))
  (`/Engine/EditorBlueprintResources/StandardMacros.IncrementInt` (`self.Snapcount`)))

(fn `ToggleRecording`
  (bind _recordings (`self.Recordings`))
  (set `self.CurrentRecordTime` 0.0)
  (bind _output_get (set `self.IsRecording` (not (`self.IsRecording`))))
  (if (not _output_get)
    (`self.SaveRecording` _recordings))
  (`KismetArrayLibrary.Array_Clear` _recordings))

(fn `UserConstructionScript`
  (set `self.VRBounds` (`SteamVRChaperoneComponent.GetBounds` (`self.SteamVRChaperone`))))