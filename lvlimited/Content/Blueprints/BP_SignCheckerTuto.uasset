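; BP_SignCheckerTuto is a tutorial actor that checks whether the player's hand sign matches the letter being taught.
; It caches the BP_Hands pawn on BeginPlay and polls its current letter every Tick.
; CheckSign maps BP_GameModeTuto's tutorial state to A, B, C, L or V, and a match calls OnLetterFinished.
; A pause timer counts down and resets on matches, but never gates detection here.
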(event `self.ReceiveBeginPlay`
  (bind _asbp_hands (cast `/Game/Blueprints/Characters/BP_Hands` (`GameplayStatics.GetPlayerPawn` 0)))
  (set `self.Player` _asbp_hands))

(event `self.ReceiveTick`
  (params (DeltaSeconds :type "Float (single-precision)"))
  (bind _player (`self.Player`))
  (if (`KismetSystemLibrary.IsValid` _player)
    (set `self.CurrentPauseTime` (- (`self.CurrentPauseTime`) DeltaSeconds))
    (if (`self.CheckSign` (`/Game/Blueprints/Characters/BP_Hands.CurrentLetter` _player))
      (set `self.CurrentPauseTime` (`self.DetectionPauseTime`))
      (bind _asbp_game_mode_tuto (cast `/Game/Blueprints/Gameplay/BP_GameModeTuto` (`GameplayStatics.GetGameMode`)))
      (`/Game/Blueprints/Gameplay/BP_GameModeTuto.OnLetterFinished` _asbp_game_mode_tuto))))

(fn `CheckSign`
  (params (Sign :type String))
  (returns (Valid :type Boolean))
  (locals (Result :type Boolean) (StateLetter :type String))
  (bind _asbp_game_mode_tuto (cast `/Game/Blueprints/Gameplay/BP_GameModeTuto` (`GameplayStatics.GetGameMode`)))
  (switch `/Game/Blueprints/Gameplay/TutorialStates` (`/Game/Blueprints/Gameplay/BP_GameModeTuto.Tuto` _asbp_game_mode_tuto)
    (:`NewEnumerator0`
      (set `local.StateLetter` "A"))
    (:`NewEnumerator1`
      (set `local.StateLetter` "B"))
    (:`NewEnumerator2`
      (set `local.StateLetter` "C"))
    (:`NewEnumerator3`
      (set `local.StateLetter` "L"))
    (:`NewEnumerator4`
      (set `local.StateLetter` "V")))
  (return (`KismetStringLibrary.EqualEqual_StrStr` (`local.StateLetter`) Sign)))

(fn `UserConstructionScript`)