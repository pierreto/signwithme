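; VR player character that recognises hand-gesture letters (A, L, V) and has hit points with an invincibility flag.
; Each tick it reads the right hand's letter, records its history and hold count, displays it as text and stores hand velocities.
; Helpers attach camera-facing widget actors and find nearest actors.
; Two-handed fireball dispatch exists but is never called here; its gesture detection and the countdown functions are unimplemented stubs.
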(event `self.ReceiveBeginPlay`
  ;[1 1 1] Set Character Start Attributes
  (set `self.LetterHoldLength` 0)
  (`HeadMountedDisplayFunctionLibrary.SetTrackingOrigin` "Floor"))

(event `self.ReceiveAnyDamage`
  (params (Damage :type "Float (single-precision)") (DamageType :type "DamageType Object Reference") (InstigatedBy :type "Controller Object Reference") (DamageCauser :type "Actor Object Reference"))
  ;[1 1 1] Damage
  (if (not (`self.Invincible`))
    (set `self.HitPoints` (- (`self.HitPoints`) Damage))))

(event `Key|Q`
  (params (Key :type "Key Structure"))
  ;[1 1 1] Quit
  (:`Pressed`
    (`KismetSystemLibrary.QuitGame` null "Quit")))

(event `self.ReceiveTick`
  (params (DeltaSeconds :type "Float (single-precision)"))
  ;[1 1 1] Detect gestures
  (set `self.Delta` DeltaSeconds)
  (bind _detection (`self.DetectLetter` (`self.HandR`)))
  (bind _output_get (set `self.CurrentLetter` _detection))
  (if (== _output_get (`self.LastLetter`))
    (`/Engine/EditorBlueprintResources/StandardMacros.IncrementInt` (`self.LetterHoldLength`)
      (:`  `
        _)))
  (`KismetArrayLibrary.Array_Add` (`self.LettersOverTime`) _output_get)
  (`TextRenderComponent.K2_SetText` (`self.TextRender`) (`KismetTextLibrary.Conv_StringToText` (`self.CurrentLetter`)))
  (set `self.LastLetter` (`self.CurrentLetter`))
  (`/Game/Blueprints/Gestuelles/Hand.StoreHandVelocities` (`self.HandR`) (`self.Delta`)))

(fn `DestroyAttachedWidget`
  (params (WidgetClass :type "Actor Class Reference"))
  (bind _outactors (`GameplayStatics.GetAllActorsOfClass` WidgetClass))
  (for _array_element _outactors
    (`self.K2_DetachFromActor` _array_element "KeepRelative" "KeepRelative" "KeepRelative")
    (`self.K2_DestroyActor` _array_element)))

(fn `DestroyWidget`)

(fn `DetectLetter`
  (params (Hand :type "/Game/Blueprints/Gestuelles/Hand Object Reference"))
  (returns (Detection :type String))
  (locals (OutputLetter :type String) (NewLocalVar_0 :type Boolean))
  (if (`/Game/Blueprints/Gestuelles/Hand.DetectA` Hand)
    (set `local.OutputLetter` "A")
    (elif (`/Game/Blueprints/Gestuelles/Hand.DetectL` Hand)
      (set `local.OutputLetter` "L")
      (elif (`/Game/Blueprints/Gestuelles/Hand.DetectV` Hand)
        (set `local.OutputLetter` "V")
        (else
          (set `local.OutputLetter` "")))))
  (return (`local.OutputLetter`)))

(fn `GetClosestActor`
  (params (ObjectClass :type "Actor Class Reference"))
  (returns (ClosestActor :type "Actor Object Reference"))
  (locals (smallestDistance :type "Float (double-precision)" :default 999999.0) (closeActor :type "Actor Object Reference"))
  (bind _outactors (`GameplayStatics.GetAllActorsOfClass` ObjectClass))
  (for _array_element _outactors
    (bind _returnvalue (`self.GetDistanceTo` _array_element))
    (if (< _returnvalue (`local.smallestDistance`))
      (set `local.closeActor` _array_element)
      (set `local.smallestDistance` _returnvalue)))
  (return (`local.closeActor`)))

(fn `GetFireballScale`)

(fn `HandleDoubleHandGestures`
  (params (DeltaTime :type "Float (double-precision)"))
  (returns (Detected :type Boolean))
  (locals (_Detected :type Boolean :default true))
  (bind _shootdirection (`self.DoubleHandGestures` DeltaTime)
    (:`OnShootFIreball`
      (`self.ShootFireballServer` _shootdirection))
    (:`OnFinalFireball`
      (`self.MoveDoubleFireball`))
    (:`OnGrowFireball`
      (`self.GrowFireball`))
    (:`OnStopFireball`
      (`self.CancelFireball`)
      (set `local._Detected` false :!label _label))
    (:`OnSpawnFireball`
      (`self.SpawnFireballDoubleHand`))
    (:`Other`
      (goto _label)))
  (return (`local._Detected`)))

(fn `ShowCountdown`
  (locals (RoundValue :type Integer :default -1)))

(fn `ShowWidget`
  (params (ActorClass :type "Actor Class Reference"))
  (returns (CreatedWidget :type "Actor Object Reference"))
  (locals (UpDistance :type "Float (double-precision)" :default -10.0) (ForwardDistance :type "Float (double-precision)" :default 150.0))
  (bind _returnvalue_roll (`KismetMathLibrary.BreakRotator` (`self.K2_GetActorRotation`)))
  (bind _camera (`self.Camera`))
  (bind (_returnvalue_roll_2 _returnvalue_pitch _returnvalue_yaw) (`KismetMathLibrary.BreakRotator` (`SceneComponent.K2_GetComponentRotation` _camera)))
  (bind _returnvalue (`KismetMathLibrary.MakeRotator` 0.0 _returnvalue_pitch _returnvalue_yaw))
  (bind (_returnvalue_roll_3 _returnvalue_pitch_2 _returnvalue_yaw_2) (`KismetMathLibrary.BreakRotator` (`KismetMathLibrary.FindLookAtRotation` (`self.K2_GetActorLocation` (`self.WidgetActor`)) (`SceneComponent.K2_GetComponentLocation` _camera))))
  (bind _returnvalue_2 (`|SpawnActorFromClass` ActorClass (`KismetMathLibrary.MakeTransform` (0.0 0.0 0.0) (struct) (0.1 0.1 0.1)) "Undefined" "OverrideRootScale" null null))
  (bind _output_get (set `self.WidgetActor` _returnvalue_2))
  (`self.K2_SetActorLocation` _output_get (+ (`SceneComponent.K2_GetComponentLocation` _camera) (+ (* (`KismetMathLibrary.GetForwardVector` _returnvalue) (`local.ForwardDistance`)) (* (`KismetMathLibrary.GetUpVector` _returnvalue) (`local.UpDistance`)))) false false)
  (`self.K2_SetActorRotation` _output_get (`KismetMathLibrary.MakeRotator` _returnvalue_roll _returnvalue_pitch_2 _returnvalue_yaw_2) false)
  (`SceneComponent.SetVisibility` (`Actor.RootComponent` (`self.WidgetActor`)) true false)
  (`self.K2_AttachToComponent` (`self.WidgetActor`) (`self.Camera`) "None" "KeepWorld" "KeepWorld" "KeepWorld" false)
  (return _returnvalue_2))

(fn `StartCountdown`
  (locals (ForwardDistance :type "Float (double-precision)" :default 100.0)))

(fn `UserConstructionScript`
  (set `self.VRBounds` (`SteamVRChaperoneComponent.GetBounds` (`self.SteamVRChaperone`))))