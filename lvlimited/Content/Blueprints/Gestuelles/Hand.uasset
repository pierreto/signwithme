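; Hand component for one side of a motion-capture glove user, providing gesture detection, hand dynamics and glove vibration.
; Finger socket positions on a child skeletal mesh feed distance and direction tests for open hand, pointing index and A, L, V signs, alongside orientation checks.
; Tick stores a short rolling window of locations and frame times for on-demand average velocity.
; Continuous vibration re-sends commands once per second, since per-tick sends hang Unreal.
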(event `self.ReceiveBeginPlay`
  ;[1 1 1] Set SkeletalMesh Reference and check for ownership
  (bind _asskeletal_mesh_component (cast `SkeletalMeshComponent` (`|GetArrayItem` (`self.GetChildrenComponents` true) 1)))
  (set `self.HandSkeleton` _asskeletal_mesh_component))

(event `self.ReceiveTick`
  (params (DeltaSeconds :type "Float (single-precision)"))
  (set `self.Delta` DeltaSeconds)
  ;[1 1 1] Store hand location so we can compute dynamics on demand
  (`self.StoreHandLocation` (`self.Delta`)))

(fn `DetectA`
  (returns (IsClosed :type Boolean))
  (bind _center (`self.GetHandCenter`))
  (bind (_thumb _index _middle _ring _pinky) (`self.GetFingerTips`))
  (return (and (> (`KismetMathLibrary.VSize` (- _center _thumb)) 3.0) (< (`KismetMathLibrary.VSize` (- _center _index)) (`self.ClosedFistRadius`)) (< (`KismetMathLibrary.VSize` (- _center _middle)) (`self.ClosedFistRadius`)) (< (`KismetMathLibrary.VSize` (- _center _ring)) (`self.ClosedFistRadius`)) (< (`KismetMathLibrary.VSize` (- _center _pinky)) (`self.ClosedFistRadius`)) (> (`KismetMathLibrary.Dot_VectorVector` (`self.GetFingerVector` "Thumb") (`self.GetRightVector` (`self.HandSkeleton`))) 0.5))))

(fn `DetectL`
  (returns (Detected :type Boolean))
  (bind _center (`self.GetHandCenter`))
  (bind (_thumb _index _middle _ring _pinky) (`self.GetFingerTips`))
  (return (and (> (`KismetMathLibrary.VSize` (- _center _thumb)) (`self.OpenedHandRadius`)) (> (`KismetMathLibrary.VSize` (- _center _index)) (`self.OpenedHandRadius`)) (< (`KismetMathLibrary.VSize` (- _center _middle)) (`self.ClosedFistRadius`)) (< (`KismetMathLibrary.VSize` (- _center _ring)) (`self.ClosedFistRadius`)) (< (`KismetMathLibrary.VSize` (- _center _pinky)) (`self.ClosedFistRadius`)))))

(fn `DetectV`
  (returns (Detected :type Boolean))
  (bind _center (`self.GetHandCenter`))
  (bind (_thumb _index _middle _ring _pinky) (`self.GetFingerTips`))
  (return (and (< (`KismetMathLibrary.VSize` (- _center _thumb)) (`self.ClosedFistRadius`)) (> (`KismetMathLibrary.VSize` (- _center _index)) (`self.OpenedHandRadius`)) (> (`KismetMathLibrary.VSize` (- _center _middle)) (`self.OpenedHandRadius`)) (< (`KismetMathLibrary.VSize` (- _center _ring)) (`self.ClosedFistRadius`)) (< (`KismetMathLibrary.VSize` (- _center _pinky)) (`self.ClosedFistRadius`)))))

(fn `GetFingerTip`
  (params (Finger :type Text))
  (returns (FingerTip :type "Vector Structure"))
  (locals (FingerTipResult :type "Vector Structure"))
  (switch `string` (`KismetTextLibrary.Conv_TextToString` Finger)
    (:`Default`
      (set `local.FingerTipResult` (`self.GetSocketLocation` (`self.HandSkeleton`) (`KismetStringLibrary.Conv_StringToName` (`KismetTextLibrary.Conv_TextToString` (`|FormatText` "Human_{Hand}InHand{Finger}4" (`self.HandSide`) Finger))))))
    (:`Thumb`
      (set `local.FingerTipResult` (`self.GetSocketLocation` (`self.HandSkeleton`) (`KismetStringLibrary.Conv_StringToName` (`KismetTextLibrary.Conv_TextToString` (`|FormatText` "Human_{Hand}Hand{Finger}4" (`self.HandSide`) Finger)))))))
  (return (`local.FingerTipResult`)))

(fn `GetFingerTips`
  (returns (Thumb :type "Vector Structure") (Index :type "Vector Structure") (Middle :type "Vector Structure") (Ring :type "Vector Structure") (Pinky :type "Vector Structure"))
  (return (`self.GetFingerTip` "Thumb") (`self.GetFingerTip` "Index") (`self.GetFingerTip` "Middle") (`self.GetFingerTip` "Ring") (`self.GetFingerTip` "Pinky")))

(fn `GetFingerVector`
  (params (Finger :type Text))
  (returns (Direction :type "Vector Structure"))
  (locals (Thumb :type Boolean))
  (bind _handskeleton (`self.HandSkeleton`))
  (bind _handside (`self.HandSide`))
  (bind _handskeleton_2 (`self.HandSkeleton`))
  (bind _handside_2 (`self.HandSide`))
  (switch `string` (`KismetTextLibrary.Conv_TextToString` Finger)
    (:`Default`
      _)
    (:`Thumb`
      (bind _output_get (set `local.Thumb` true))))
  (return (select `bool` _output_get :`false` (`KismetMathLibrary.Normal` (- (`self.GetSocketLocation` _handskeleton_2 (`KismetStringLibrary.Conv_StringToName` (`KismetTextLibrary.Conv_TextToString` (`|FormatText` "Human_{Hand}InHand{Finger}4" _handside Finger)))) (`self.GetSocketLocation` _handskeleton_2 (`KismetStringLibrary.Conv_StringToName` (`KismetTextLibrary.Conv_TextToString` (`|FormatText` "Human_{Hand}InHand{Finger}1" _handside Finger)))))) :`true` (`KismetMathLibrary.Normal` (- (`self.GetSocketLocation` _handskeleton (`KismetStringLibrary.Conv_StringToName` (`KismetTextLibrary.Conv_TextToString` (`|FormatText` "Human_{Hand}Hand{Finger}4" _handside_2 Finger)))) (`self.GetSocketLocation` _handskeleton (`KismetStringLibrary.Conv_StringToName` (`KismetTextLibrary.Conv_TextToString` (`|FormatText` "Human_{Hand}Hand{Finger}1" _handside_2 Finger)))))))))

(fn `GetHandCenter`
  (returns (Center :type "Vector Structure"))
  (return (/ (+ (.location (`self.GetSocketTransform` (`self.HandSkeleton`) (`KismetStringLibrary.Conv_StringToName` (`KismetTextLibrary.Conv_TextToString` (`|FormatText` "Human_{Hand}InHandMiddle1" (`self.HandSide`)))) "RTS_World")) (.location (`self.GetSocketTransform` (`self.HandSkeleton`) (`KismetStringLibrary.Conv_StringToName` (`KismetTextLibrary.Conv_TextToString` (`|FormatText` "Human_{Hand}InHandMiddle" (`self.HandSide`)))) "RTS_World"))) 2)))

(fn `GetMiddleFingerCenter`
  (returns (Location :type "Vector Structure"))
  (bind _returnvalue_location (`KismetMathLibrary.BreakTransform` (`self.GetSocketTransform` (`self.HandSkeleton`) (`KismetStringLibrary.Conv_StringToName` (`KismetTextLibrary.Conv_TextToString` (`|FormatText` "Human_{Hand}InHandMiddle2" (`self.HandSide`)))) "RTS_World")))
  (return _returnvalue_location))

(fn `GetPalmVector`
  (returns (Vector :type "Vector Structure"))
  (return (* (`self.GetUpVector` (`self.HandSkeleton`)) -1)))

(fn `GetShootDirection`
  (returns (Direction :type "Vector Structure"))
  (return (`KismetMathLibrary.Normal` (- (`self.GetHandCenter`) (`self.GetRightShoulder`)))))

(fn `GetVelocity`
  (returns (Velocity :type "Vector Structure"))
  (locals (Velocities :type "Array of Vector Structure"))
  ;[1 1 1] Compute average velocity
  (if (> (`KismetArrayLibrary.Array_Length` (`self.Locations`)) 1)
    (for (_array_element _array_index) (`self.Locations`)
      (if (> _array_index 0)
        (`KismetArrayLibrary.Array_Add` (`local.Velocities`) (/ (- _array_element (`|GetArrayItem` (`self.Locations`) (- _array_index 1))) (`|GetArrayItem` (`self.Times`) _array_index)))))
    (else
      (`KismetArrayLibrary.Array_Add` (`local.Velocities`))))
  (return (`KismetMathLibrary.GetVectorArrayAverage` (`local.Velocities`))))

(fn `HandPointingDown`
  (returns (IsPointingDown :type Boolean))
  (bind (_returnvalue_roll _returnvalue_pitch) (`KismetMathLibrary.BreakRotator` (`self.K2_GetComponentRotation` (`self.HandSkeleton`))))
  (return (and (<= _returnvalue_roll 30.0) (>= _returnvalue_roll -30.0) (<= _returnvalue_pitch 30.0) (>= _returnvalue_pitch -30.0))))

(fn `HandPointingUp`
  (returns (IsPointingDown :type Boolean))
  (bind _handskeleton (`self.HandSkeleton`))
  (bind _returnvalue_roll (`KismetMathLibrary.BreakRotator` (`self.K2_GetComponentRotation` _handskeleton)))
  (return (and (<= (`.Pitch` (`KismetMathLibrary.GetYawPitchFromVector` (`self.GetUpVector` _handskeleton))) -60.0) (>= (`KismetMathLibrary.Abs` _returnvalue_roll) 140.0))))

(fn `IsHandOpen`
  (returns (IsOpened :type Boolean))
  (locals (Detection :type Integer))
  (bind _center (`self.GetHandCenter`))
  (bind (_thumb _index _middle _ring _pinky) (`self.GetFingerTips`))
  (return (>= (+ (`KismetMathLibrary.Conv_BoolToInt` (> (`KismetMathLibrary.VSize` (- _center _index)) (`self.OpenedHandRadius`))) (`KismetMathLibrary.Conv_BoolToInt` (> (`KismetMathLibrary.VSize` (- _center _middle)) (`self.OpenedHandRadius`))) (`KismetMathLibrary.Conv_BoolToInt` (> (`KismetMathLibrary.VSize` (- _center _ring)) (`self.OpenedHandRadius`))) (`KismetMathLibrary.Conv_BoolToInt` (> (`KismetMathLibrary.VSize` (- _center _pinky)) (`self.OpenedHandRadius`)))) 3)))

(fn `IsIndexPointing`
  (returns (Detected :type Boolean))
  (bind _center (`self.GetHandCenter`))
  (bind (_thumb _index _middle _ring _pinky) (`self.GetFingerTips`))
  (return (and (> (`KismetMathLibrary.VSize` (- _center _index)) (`self.OpenedHandRadius`)) (< (`KismetMathLibrary.VSize` (- _center _middle)) (`self.ClosedFistRadius`)) (< (`KismetMathLibrary.VSize` (- _center _ring)) (`self.ClosedFistRadius`)) (< (`KismetMathLibrary.VSize` (- _center _pinky)) (`self.ClosedFistRadius`)))))

(fn `StopVibration`
  ;[1 1 1] Stops glove vibration. Unreal hangs if we send commands on each Tick...
  (if (`self.IsVibrating`)
    (switch `string` (`KismetTextLibrary.Conv_TextToString` (`self.HandSide`))
      (:`Left`
        (`MotionCaptureFunctionLibrary.VibrateLeftGlove` 0))
      (:`Right`
        (`MotionCaptureFunctionLibrary.VibrateRightGlove` 0)))
    (set `self.IsVibrating` false)))

(fn `StoreHandLocation`
  (params (deltaT :type "Float (double-precision)"))
  ;[1 1 1] Store Hand Velocity To Compute Average Later
  (`KismetArrayLibrary.Array_Add` (`self.Times`) deltaT)
  (bind _returnvalue (`KismetArrayLibrary.Array_Add` (`self.Locations`) (`self.K2_GetComponentLocation` (`self.HandSkeleton`))))
  (if (> _returnvalue 10)
    (`KismetArrayLibrary.Array_Remove` (`self.Locations`))
    (`KismetArrayLibrary.Array_Remove` (`self.Times`))))

(fn `StoreHandVelocities`
  (params (deltaT :type "Float (double-precision)"))
  (bind _handvelocities (`self.HandVelocities`))
  ;[1 1 1] Store Hand Velocity To Compute Average Later
  (`KismetArrayLibrary.Array_Add` _handvelocities (/ (- (`self.K2_GetComponentLocation` (`self.HandSkeleton`)) (`self.LastHandPos`)) deltaT))
  (if (> (`KismetArrayLibrary.Array_Length` _handvelocities) 10)
    (`KismetArrayLibrary.Array_Remove` (`self.HandVelocities`))
    (set `self.LastHandPos` (`self.K2_GetComponentLocation` (`self.HandSkeleton`)))))

(fn `VibrateGlove`
  (params (Milliseconds :type Integer))
  (switch `string` (`KismetTextLibrary.Conv_TextToString` (`self.HandSide`))
    (:`Left`
      (`MotionCaptureFunctionLibrary.VibrateLeftGlove` Milliseconds))
    (:`Right`
      (`MotionCaptureFunctionLibrary.VibrateRightGlove` Milliseconds))))

(fn `VibrateGloveContinuous`
  ;[1 1 1] Send a vibrate command every second. MotionCaptureComponent does not like vibrating on each tick (Unreal hangs)
  (if (`self.IsVibrating`)
    (bind _output_get (set `self.TimeSinceLastVibration` (+ (`self.Delta`) (`self.TimeSinceLastVibration`))))
    (if (>= _output_get 1.0)
      (switch `string` (`KismetTextLibrary.Conv_TextToString` (`self.HandSide`)) :!label _label
        (:`Left`
          (`MotionCaptureFunctionLibrary.VibrateLeftGlove` 1000))
        (:`Right`
          (`MotionCaptureFunctionLibrary.VibrateRightGlove` 1000)))
      (set `self.TimeSinceLastVibration` 0.0)
      (set `self.IsVibrating` true))
    (else
      (goto _label))))