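; BP_SignBlockLevel3 is a moving block that shows a sign's name and plays its recording through a child BP_Replayer, with the left side hidden.
; On BeginPlay a timeline carries Tackroot along a spline while rolling it, then Tick drives the actor forward.
; Crossing a hardcoded world Y threshold destroys it, resets the game mode's combo and clears the word in BP_WordSpawnerAndChecker.
; MakeGreen and MakeRed create dynamic material instances on the mesh.
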(event `self.ReceiveBeginPlay`
  (bind _tackroot (`self.tackroot`))
  (bind _spline (`self.Spline`))
  (bind (_x _y _z) (`KismetMathLibrary.BreakRotIntoAxes` (`SceneComponent.K2_GetComponentRotation` (`self.tackroot`))))
  (bind _asbp_replayer (cast `/Game/Blueprints/Record/BP_Replayer` (`ChildActorComponent.ChildActor` (`self.Replayer`))))
  (bind _output_get (set `self.ReplayerRef` _asbp_replayer))
  (`/Game/Blueprints/Record/BP_Replayer.HideLeft` _output_get)
  (bind (_direction _newtrack_0) (`Timeline|Timeline_0` :!via `PlayFromStart`)
    (:`Update`
      (bind _returnvalue (* _newtrack_0 (`SplineComponent.GetSplineLength` _spline)))
      (`SceneComponent.K2_SetWorldTransform` _tackroot (`KismetMathLibrary.MakeTransform` (`SplineComponent.GetLocationAtDistanceAlongSpline` _spline _returnvalue "World") (`KismetMathLibrary.MakeRotator` (+ (.x _x) _returnvalue) (.y _y) (.z _z)) (`SceneComponent.K2_GetComponentScale` _tackroot)) false false))
    (:`Finished`
      (set `self.Initialized` true))))

(event `self.ReceiveTick`
  (params (DeltaSeconds :type "Float (single-precision)"))
  (bind _returnvalue (+ (`self.K2_GetActorLocation`) (* (* (`self.GetActorForwardVector`) (`self.Speed`)) DeltaSeconds)))
  (if (`self.Initialized`)
    (`self.K2_SetActorLocation` _returnvalue)
    (if (>= (.y _returnvalue) -90.0)
      (`self.Collision`))))

(fn `Collision`
  (`self.K2_DestroyActor`)
  (bind _asbp_game_mode (cast `/Game/Blueprints/Gameplay/BP_GameMode` (`GameplayStatics.GetGameMode`)))
  (`/Game/Blueprints/Gameplay/BP_GameMode.ResetCombo` _asbp_game_mode)
  (bind _outactors (`GameplayStatics.GetAllActorsOfClass` "/Game/Blueprints/SceneActors/BP_WordSpawnerAndChecker.BP_WordSpawnerAndChecker_C"))
  (`/Game/Blueprints/SceneActors/BP_WordSpawnerAndChecker.ClearWord` (`|GetArrayItem` _outactors)))

(fn `MakeGreen`
  (`PrimitiveComponent.CreateDynamicMaterialInstance` (`self.StaticMesh`) 0 "/Game/Assets/Material/EGreen.EGreen" "None"))

(fn `MakeRed`
  (`PrimitiveComponent.CreateDynamicMaterialInstance` (`self.StaticMesh`) 0 null "None"))

(fn `SetSignText`
  (bind _returnvalue (`|GetEnumeratorNameAsString` (`self.Sign`)))
  (`TextRenderComponent.K2_SetText` (`self.SignText`) (`KismetTextLibrary.Conv_StringToText` _returnvalue))
  (bind (_recordings _success) (`/Game/Blueprints/Record/BP_Replayer.LoadRecording` (`self.ReplayerRef`) _returnvalue))
  (if _success
    (`/Game/Blueprints/Record/BP_Replayer.Play` (`self.ReplayerRef`) _recordings)))

(fn `UserConstructionScript`)