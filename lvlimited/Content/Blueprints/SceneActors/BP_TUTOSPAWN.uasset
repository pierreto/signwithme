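; Tutorial spawn actor that builds a set of letter sign blocks when play begins.
; Each static mesh component tagged "Letter" gets a BP_SignBlockLevel0 spawned above it along its up vector, yawed relative to a central mesh and rolled 180 degrees.
; Each sign is whitened, takes the component's first tag as both text and actor tag, then attaches to this actor.
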(event `self.ReceiveBeginPlay`
  (bind (_returnvalue_x _returnvalue_y) (`KismetMathLibrary.BreakVector` (`SceneComponent.K2_GetComponentLocation` (`self.StaticMeshComponent013`))))
  (for _array_element (`self.GetComponentsByTag` "/Script/Engine.StaticMeshComponent" "Letter")
    (bind _returnvalue (+ (* (`SceneComponent.GetUpVector` _array_element) 200.0) (.location (`SceneComponent.K2_GetComponentToWorld` _array_element))))
    (bind _returnvalue_2 (`|SpawnActorFromClass` "/Game/Blueprints/SceneActors/BP_SignBlockLevel0.BP_SignBlockLevel0_C" (`KismetMathLibrary.MakeTransform` _returnvalue (`KismetMathLibrary.ComposeRotators` (`KismetMathLibrary.FindLookAtRotation` _returnvalue (`KismetMathLibrary.MakeVector` _returnvalue_x _returnvalue_y (.z _returnvalue))) (struct :`Yaw` 180.0))) "Undefined" "OverrideRootScale" null null))
    (`/Game/Blueprints/SceneActors/BP_SignBlockLevel0.WhiteMeDaddy` _returnvalue_2)
    (bind _output (`|GetArrayItem` (`ActorComponent.ComponentTags` _array_element)))
    (`/Game/Blueprints/SceneActors/BP_SignBlockLevel0.SetSignText2` _returnvalue_2 (`KismetStringLibrary.Conv_NameToString` _output))
    (`KismetArrayLibrary.Array_Add` (`Actor.Tags` _returnvalue_2) _output)
    (`self.K2_AttachToActor` _returnvalue_2 self "None" "KeepWorld" "KeepWorld" "KeepWorld" true)))

(fn `UserConstructionScript`)