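; BP_SignBlockStatic is a sign block actor that shows the name of its Sign enum as text, set on BeginPlay.
; Its Collision function removes the first entry from BP_Spawner's CurrentSignBlocks, resets the game mode's combo and destroys the block.
; The removal targets index 0 of the first spawner found, regardless of which block collided.
; Replayer logic for caching the child actor and playing the sign's recording is present but disconnected.
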(event `self.ReceiveBeginPlay`
  (`self.SetSignText`))

(event `self.ReceiveTick`
  (params (DeltaSeconds :type "Float (single-precision)")))

(fn `Collision`
  (bind _outactors (`GameplayStatics.GetAllActorsOfClass` "/Game/Blueprints/SceneActors/BP_Spawner.BP_Spawner_C"))
  (`KismetArrayLibrary.Array_Remove` (`/Game/Blueprints/SceneActors/BP_Spawner.CurrentSignBlocks` (`|GetArrayItem` _outactors)))
  (bind _asbp_game_mode (cast `/Game/Blueprints/Gameplay/BP_GameMode` (`GameplayStatics.GetGameMode`)))
  (`/Game/Blueprints/Gameplay/BP_GameMode.ResetCombo` _asbp_game_mode)
  (`self.K2_DestroyActor`))

(fn `SetSignText`
  (`TextRenderComponent.K2_SetText` (`self.SignText`) (`KismetTextLibrary.Conv_StringToText` (`|GetEnumeratorNameAsString` (`self.Sign`)))))

(fn `UserConstructionScript`)