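; Lounge pillar scene actor that displays a letter and carries tagged lights with green and red functions.
; On BeginPlay it attaches to the first BP_TUTOSPAWN found, keeping its world transform.
; The construction script writes LetterV to the Letter text, and SetText replaces it.
; Greenlight and Redlight create dynamic instances of EGreen or ERed per "Light"-tagged mesh, but never assign them to the meshes.
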(event `self.ReceiveBeginPlay`
  (bind _outactors (`GameplayStatics.GetAllActorsOfClass` "/Game/Blueprints/SceneActors/BP_TUTOSPAWN.BP_TUTOSPAWN_C"))
  (`self.K2_AttachToActor` (`|GetArrayItem` _outactors) "None" "KeepWorld" "KeepWorld" "KeepWorld"))

(fn `Greenlight`
  (for _array_element (`self.GetComponentsByTag` "/Script/Engine.StaticMeshComponent" "Light")
    (`KismetMaterialLibrary.CreateDynamicMaterialInstance` _array_element "/Game/Assets/Material/EGreen.EGreen")))

(fn `Redlight`
  (for _array_element (`self.GetComponentsByTag` "/Script/Engine.StaticMeshComponent" "Light")
    (`KismetMaterialLibrary.CreateDynamicMaterialInstance` _array_element "/Game/Assets/Material/ERed.ERed")))

(fn `SetText`
  (params (NewParam :type String))
  (`TextRenderComponent.K2_SetText` (`self.Letter`) (`KismetTextLibrary.Conv_StringToText` NewParam)))

(fn `UserConstructionScript`
  (`TextRenderComponent.K2_SetText` (`self.Letter`) (`KismetTextLibrary.Conv_StringToText` (`self.LetterV`))))