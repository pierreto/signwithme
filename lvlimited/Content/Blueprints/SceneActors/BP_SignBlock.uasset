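; BP_SignBlock is a moving block that displays a sign's name and plays back that sign's recording through a child BP_Replayer with its left side hidden.
; It moves along its forward vector each tick, and SetSignText uses the Sign enum name for both the label and recording lookup.
; Overlapping BP_Hands removes the first entry from the spawner's CurrentSignBlocks, resets the game mode's combo and destroys the block.
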(event `self.ReceiveBeginPlay`
  (bind _asbp_replayer (cast `/Game/Blueprints/Record/BP_Replayer` (`ChildActorComponent.ChildActor` (`self.Replayer`))))
  (bind _output_get (set `self.ReplayerRef` _asbp_replayer))
  (`/Game/Blueprints/Record/BP_Replayer.HideLeft` _output_get))

(event `self.ReceiveTick`
  (params (DeltaSeconds :type "Float (single-precision)"))
  (`self.K2_SetActorLocation` (+ (`self.K2_GetActorLocation`) (* (* (`self.GetActorForwardVector`) (`self.Speed`)) DeltaSeconds))))

(event `self.ReceiveActorBeginOverlap`
  (params (OtherActor :type "Actor Object Reference"))
  (cast `/Game/Blueprints/Characters/BP_Hands` OtherActor)
  (`self.Collision`))

(fn `Collision`
  (bind _outactors (`GameplayStatics.GetAllActorsOfClass` "/Game/Blueprints/SceneActors/BP_Spawner.BP_Spawner_C"))
  (`KismetArrayLibrary.Array_Remove` (`/Game/Blueprints/SceneActors/BP_Spawner.CurrentSignBlocks` (`|GetArrayItem` _outactors)))
  (bind _asbp_game_mode (cast `/Game/Blueprints/Gameplay/BP_GameMode` (`GameplayStatics.GetGameMode`)))
  (`/Game/Blueprints/Gameplay/BP_GameMode.ResetCombo` _asbp_game_mode)
  (`self.K2_DestroyActor`))

(fn `SetSignText`
  (bind _returnvalue (`|GetEnumeratorNameAsString` (`self.Sign`)))
  (`TextRenderComponent.K2_SetText` (`self.SignText`) (`KismetTextLibrary.Conv_StringToText` _returnvalue))
  (bind (_recordings _success) (`/Game/Blueprints/Record/BP_Replayer.LoadRecording` (`self.ReplayerRef`) _returnvalue))
  (if _success
    (`/Game/Blueprints/Record/BP_Replayer.Play` (`self.ReplayerRef`) _recordings)))

(fn `UserConstructionScript`)