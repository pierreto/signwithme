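; BP_Spawner spawns BP_SignBlock actors from a shuffled sign queue during the Level 1 game state.
; BeginPlay fills the queue with a set number of each sign.
; Tick spawns blocks on a countdown, giving each the queue's front sign, which stays queued until DestroyCurrentSign.
; DestroyCurrentSign removes the oldest block and front sign, adds score and combo through BP_GameMode, and ends the level when the queue empties.
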(event `self.ReceiveBeginPlay`
  (bind _asbp_game_state (cast `/Game/Blueprints/Gameplay/BP_GameState` (`GameplayStatics.GetGameState`)))
  (set `self.GameStateRef` _asbp_game_state)
  (set `self.CurrentTimer` (`self.SpawnSpeed`))
  (`KismetArrayLibrary.Array_Clear` (`self.CurrentSignBlocks`))
  (for _index (range (enumcount `/Game/Blueprints/SceneActors/E_Signs`))
    (for _ (range (`self.Number`))
      (`KismetArrayLibrary.Array_Add` (`self.Signs`) (`KismetMathLibrary.Conv_IntToByte` _index))))
  (`KismetArrayLibrary.Array_Shuffle` (`self.Signs`)))

(event `self.ReceiveTick`
  (params (DeltaSeconds :type "Float (single-precision)"))
  (switch `/Game/Blueprints/Gameplay/GameStates` (`/Game/Blueprints/Gameplay/BP_GameState.GameState` (`self.GameStateRef`))
    (:`NewEnumerator2`
      (if (> (`KismetArrayLibrary.Array_Length` (`self.Signs`)) 0)
        (bind _output_get (set `self.CurrentTimer` (- (`self.CurrentTimer`) DeltaSeconds)))
        (if (<= _output_get 0.0)
          (bind _returnvalue (`|SpawnActorFromClass` "/Game/Blueprints/SceneActors/BP_SignBlock.BP_SignBlock_C" (`self.GetTransform` self) "Undefined" "OverrideRootScale" null null))
          (set `/Game/Blueprints/SceneActors/BP_SignBlock.Sign` (cast `/Game/Blueprints/SceneActors/E_Signs` (`|GetArrayItem` (`self.Signs`))) _returnvalue)
          (`/Game/Blueprints/SceneActors/BP_SignBlock.SetSignText` _returnvalue)
          (set `self.CurrentTimer` (`self.SpawnSpeed`))
          (`KismetArrayLibrary.Array_Add` (`self.CurrentSignBlocks`) _returnvalue))))))

(fn `DestroyCurrentSign`
  (`self.K2_DestroyActor` (`|GetArrayItem` (`self.CurrentSignBlocks`)))
  (`KismetArrayLibrary.Array_Remove` (`self.CurrentSignBlocks`))
  (`KismetArrayLibrary.Array_Remove` (`self.Signs`))
  (bind _asbp_game_mode (cast `/Game/Blueprints/Gameplay/BP_GameMode` (`GameplayStatics.GetGameMode`)))
  (`/Game/Blueprints/Gameplay/BP_GameMode.AddScore` _asbp_game_mode)
  (`/Game/Blueprints/Gameplay/BP_GameMode.AddCombo` _asbp_game_mode)
  (if (<= (`KismetArrayLibrary.Array_Length` (`self.Signs`)) 0)
    (bind _asbp_game_mode_2 (cast `/Game/Blueprints/Gameplay/BP_GameMode` (`GameplayStatics.GetGameMode`)))
    (`/Game/Blueprints/Gameplay/BP_GameMode.LevelEnded` _asbp_game_mode_2)))

(fn `UserConstructionScript`)