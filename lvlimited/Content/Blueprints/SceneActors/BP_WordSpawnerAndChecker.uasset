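; Level 3 actor that spawns words as rows of moving sign blocks and checks the player's hand signs against them.
; When no word is active, a Tick timer spawns one BP_SignBlockLevel3 per letter of the current word.
; Tick matches BP_Hands' current letter in order, greening blocks with a pause between matches.
; Completed words score, update BP_GoalThirdLevelActor's counters and advance the index, eventually ending the level through BP_GameMode.
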(event `self.ReceiveBeginPlay`
  (bind _asbp_game_state (cast `/Game/Blueprints/Gameplay/BP_GameState` (`GameplayStatics.GetGameState`)))
  (set `self.GameStateRef` _asbp_game_state)
  (`KismetArrayLibrary.Array_Clear` (`self.CurrentSignBlocks`))
  (bind _asbp_hands (cast `/Game/Blueprints/Characters/BP_Hands` (`GameplayStatics.GetPlayerPawn` 0)))
  (set `self.Player` _asbp_hands))

(event `self.ReceiveTick`
  (params (DeltaSeconds :type "Float (single-precision)"))
  (bind (_returnvalue_location _returnvalue_rotation _returnvalue_scale) (`KismetMathLibrary.BreakTransform` (`self.GetTransform` self)))
  (set `self.CurrentPauseTime` (- (`self.CurrentPauseTime`) DeltaSeconds))
  (set `self.CurrentSpawnTime` (- (`self.CurrentSpawnTime`) DeltaSeconds))
  (if (> (`KismetArrayLibrary.Array_Length` (`self.CurrentSignBlocks`)) 0)
    (if (and (== (`/Game/Blueprints/Characters/BP_Hands.CurrentLetter` (`self.Player`)) (`|GetArrayItem` (`KismetStringLibrary.GetCharacterArrayFromString` (`self.CurrentWord`)) (`self.CurrentLetterIndex`))) (<= (`self.CurrentPauseTime`) 0.0))
      (`self.MarkGreenCurrentSign`)
      (set `self.CurrentPauseTime` (`self.PauseTime`))
      (`/Engine/EditorBlueprintResources/StandardMacros.IncrementInt` (`self.CurrentLetterIndex`)
        (:`  `
          (if (== (`KismetStringLibrary.Len` (`self.CurrentWord`)) (`self.CurrentLetterIndex`))
            (for _array_element (`self.CurrentSignBlocks`)
              (`/Game/Blueprints/SceneActors/BP_SignBlockLevel3.OnPointScored` _array_element (`self.CurrentWordIndex`)))
            (bind _outactors (`GameplayStatics.GetAllActorsOfClass` "/Game/Blueprints/SceneActors/BP_GoalThirdLevelActor.BP_GoalThirdLevelActor_C"))
            (switch `int` (`self.CurrentWordIndex`)
              (:`0`
                (bind _output (`|GetArrayItem` _outactors))
                (`/Game/Blueprints/SceneActors/BP_GoalThirdLevelActor.UpdateW1Count` _output))
              (:`1`
                (`/Game/Blueprints/SceneActors/BP_GoalThirdLevelActor.UpdateW2Count` _output))
              (:`2`
                (`/Game/Blueprints/SceneActors/BP_GoalThirdLevelActor.UpdateW3Count` _output)))
            (bind _result (`/Engine/EditorBlueprintResources/StandardMacros.IncrementInt` (`self.CurrentWordIndex`))
              (:`  `
                (set `self.WordPresent` false)
                (`KismetArrayLibrary.Array_Clear` (`self.CurrentSignBlocks`))
                (if (== _result 2)
                  (bind _asbp_game_mode (cast `/Game/Blueprints/Gameplay/BP_GameMode` (`GameplayStatics.GetGameMode`)))
                  (`/Game/Blueprints/Gameplay/BP_GameMode.LevelEnded` _asbp_game_mode))))))))
    (elif (<= (`self.CurrentSpawnTime`) 0.0)
      (set `self.CurrentLetterIndex` 0)
      (set `self.WordPresent` true)
      (for (_array_element_2 _array_index) (`KismetStringLibrary.GetCharacterArrayFromString` (`|GetArrayItem` (`self.Words`) (`self.CurrentWordIndex`)))
        (switch `string` _array_element_2
          (:`A`
            (set `self.Sign` "NewEnumerator1"))
          (:`B`
            (set `self.Sign` "NewEnumerator3"))
          (:`C`
            (set `self.Sign` "NewEnumerator4"))
          (:`L`
            (set `self.Sign` "NewEnumerator0"))
          (:`V`
            (set `self.Sign` "NewEnumerator2")))
        (bind _returnvalue (`|SpawnActorFromClass` "/Game/Blueprints/SceneActors/BP_SignBlockLevel3.BP_SignBlockLevel3_C" (`KismetMathLibrary.MakeTransform` (+ (* (`self.GetActorRightVector` self) (* _array_index 100)) _returnvalue_location) _returnvalue_rotation _returnvalue_scale) "Undefined" "OverrideRootScale" null null))
        (set `/Game/Blueprints/SceneActors/BP_SignBlockLevel3.Sign` (`self.Sign`) _returnvalue)
        (`/Game/Blueprints/SceneActors/BP_SignBlockLevel3.SetSignText` _returnvalue)
        (set `/Game/Blueprints/SceneActors/BP_SignBlockLevel3.Speed` -100.0 _returnvalue)
        (`KismetArrayLibrary.Array_Add` (`self.CurrentSignBlocks`) _returnvalue)
        (set `self.CurrentWord` (`|GetArrayItem` (`self.Words`) (`self.CurrentWordIndex`)))))))

(fn `ClearWord`
  (set `self.CurrentLetterIndex` 0)
  (set `self.WordPresent` false)
  (`KismetArrayLibrary.Array_Clear` (`self.CurrentSignBlocks`))
  (set `self.CurrentSpawnTime` (`self.SpawnTime`)))

(fn `DestroyWord`
  (`KismetArrayLibrary.Array_Clear` (`self.CurrentSignBlocks`))
  (bind _asbp_game_mode (cast `/Game/Blueprints/Gameplay/BP_GameMode` (`GameplayStatics.GetGameMode`)))
  (`/Game/Blueprints/Gameplay/BP_GameMode.AddScore` _asbp_game_mode)
  ;[1 1 1] maybe remove
  (`/Game/Blueprints/Gameplay/BP_GameMode.AddCombo` _asbp_game_mode)
  (set `self.CurrentSpawnTime` (`self.SpawnTime`)))

(fn `MarkGreenCurrentSign`
  (`KismetSystemLibrary.PrintString` "Hello")
  (`/Game/Blueprints/SceneActors/BP_SignBlockLevel3.MakeGreen` (`|GetArrayItem` (`self.CurrentSignBlocks`) (`self.CurrentLetterIndex`))))

(fn `UserConstructionScript`)