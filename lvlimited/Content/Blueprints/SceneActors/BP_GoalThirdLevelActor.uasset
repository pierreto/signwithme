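; Goal display actor for the third level, tracking three words (CAB, LAVA, BALL) built from collected letters.
; Per-word getters map a letter's sign to its slot transform, using flags to give repeated letters the next slot.
; Update functions increment "current/goal" text counters by parsing the displayed string and clamping to GoalCount.
; Show and Hide toggle the whole actor through root visibility propagation.
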(fn `GetW1Transform`
  (params (Letter :type "/Game/Blueprints/SceneActors/BP_SignBlock Object Reference"))
  (returns (Location :type "Transform Structure"))
  (locals (LetterLocation :type "Transform Structure"))
  (switch `/Game/Blueprints/SceneActors/E_Signs` (`/Game/Blueprints/SceneActors/BP_SignBlock.Sign` Letter)
    (:`NewEnumerator1`
      (set `local.LetterLocation` (`SceneComponent.K2_GetComponentToWorld` (`self.W1L2`))))
    (:`NewEnumerator3`
      (set `local.LetterLocation` (`SceneComponent.K2_GetComponentToWorld` (`self.W1L3`))))
    (:`NewEnumerator4`
      (set `local.LetterLocation` (`SceneComponent.K2_GetComponentToWorld` (`self.W1L1`)))))
  (return (`local.LetterLocation`)))

(fn `GetW2Transform`
  (params (Letter :type "/Game/Blueprints/SceneActors/BP_SignBlock Object Reference"))
  (returns (Location :type "Transform Structure"))
  (locals (LetterLocation :type "Transform Structure"))
  (switch `/Game/Blueprints/SceneActors/E_Signs` (`/Game/Blueprints/SceneActors/BP_SignBlock.Sign` Letter)
    (:`NewEnumerator1`
      (if (`self.W2L2GotTransform`)
        (set `local.LetterLocation` (`SceneComponent.K2_GetComponentToWorld` (`self.W2L4`)))
        (else
          (set `local.LetterLocation` (`SceneComponent.K2_GetComponentToWorld` (`self.W2L2`)))
          (set `self.W2L2GotTransform` true))))
    (:`NewEnumerator0`
      (if (`self.W2L1GotTransform`)
        (set `local.LetterLocation` (struct))
        (else
          (set `local.LetterLocation` (`SceneComponent.K2_GetComponentToWorld` (`self.W2L1`)))
          (set `self.W2L1GotTransform` true))))
    (:`NewEnumerator2`
      (set `local.LetterLocation` (`SceneComponent.K2_GetComponentToWorld` (`self.W2L3`)))))
  (return (`local.LetterLocation`)))

(fn `GetW3Transform`
  (params (Letter :type "/Game/Blueprints/SceneActors/BP_SignBlock Object Reference"))
  (returns (Location :type "Transform Structure"))
  (locals (LetterLocation :type "Transform Structure"))
  (switch `/Game/Blueprints/SceneActors/E_Signs` (`/Game/Blueprints/SceneActors/BP_SignBlock.Sign` Letter)
    (:`NewEnumerator1`
      (set `local.LetterLocation` (`SceneComponent.K2_GetComponentToWorld` (`self.W3L2`))))
    (:`NewEnumerator3`
      (set `local.LetterLocation` (`SceneComponent.K2_GetComponentToWorld` (`self.W3L1`))))
    (:`NewEnumerator0`
      (if (`self.W3L3GotTransform`)
        (set `local.LetterLocation` (`SceneComponent.K2_GetComponentToWorld` (`self.W3L4`)))
        (else
          (set `local.LetterLocation` (`SceneComponent.K2_GetComponentToWorld` (`self.W3L3`)))
          (set `self.W3L3GotTransform` true)))))
  (return (`local.LetterLocation`)))

(fn `Hide`
  (`SceneComponent.SetVisibility` (`self.DefaultSceneRoot`) false true))

(fn `Show`
  (`SceneComponent.SetVisibility` (`self.DefaultSceneRoot`) true true))

(fn `UpdateLetterCount`
  (params (Letter :type "/Game/Blueprints/SceneActors/BP_SignBlock Object Reference"))
  (locals (LetterToUpdate :type "TextRenderComponent Object Reference"))
  (bind _goalcount (`self.GoalCount`))
  (switch `/Game/Blueprints/SceneActors/E_Signs` (`/Game/Blueprints/SceneActors/BP_SignBlock.Sign` Letter)
    (:`NewEnumerator1`
      (set `local.LetterToUpdate` (`self.CountW1`)))
    (:`NewEnumerator3`
      (set `local.LetterToUpdate` (`self.CountW2`)))
    (:`NewEnumerator4`
      (set `local.LetterToUpdate` (`self.CountW3`)))
    (:`NewEnumerator0`
      (set `local.LetterToUpdate` null))
    (:`NewEnumerator2`
      (set `local.LetterToUpdate` null)))
  (`TextRenderComponent.K2_SetText` (`local.LetterToUpdate`) (`KismetTextLibrary.Conv_StringToText` (`KismetStringLibrary.Concat_StrStr` (`KismetStringLibrary.Conv_IntToString` (`KismetMathLibrary.Clamp` (+ (`KismetStringLibrary.Conv_StringToInt` (`KismetStringLibrary.Split` (`KismetTextLibrary.Conv_TextToString` (`TextRenderComponent.Text` (`local.LetterToUpdate`))) "/")) 1) 0 _goalcount)) "/" (`KismetStringLibrary.Conv_IntToString` _goalcount)))))

(fn `UpdateW1Count`
  (bind _goalcount (`self.GoalCount`))
  (`TextRenderComponent.K2_SetText` (`self.CountW1`) (`KismetTextLibrary.Conv_StringToText` (`KismetStringLibrary.Concat_StrStr` (`KismetStringLibrary.Conv_IntToString` (`KismetMathLibrary.Clamp` (+ (`KismetStringLibrary.Conv_StringToInt` (`KismetStringLibrary.Split` (`KismetTextLibrary.Conv_TextToString` (`TextRenderComponent.Text` (`self.CountW1`))) "/")) 1) 0 _goalcount)) "/" (`KismetStringLibrary.Conv_IntToString` _goalcount)))))

(fn `UpdateW2Count`
  (bind _goalcount (`self.GoalCount`))
  (`TextRenderComponent.K2_SetText` (`self.CountW2`) (`KismetTextLibrary.Conv_StringToText` (`KismetStringLibrary.Concat_StrStr` (`KismetStringLibrary.Conv_IntToString` (`KismetMathLibrary.Clamp` (+ (`KismetStringLibrary.Conv_StringToInt` (`KismetStringLibrary.Split` (`KismetTextLibrary.Conv_TextToString` (`TextRenderComponent.Text` (`self.CountW2`))) "/")) 1) 0 _goalcount)) "/" (`KismetStringLibrary.Conv_IntToString` _goalcount)))))

(fn `UpdateW3Count`
  (bind _goalcount (`self.GoalCount`))
  (`TextRenderComponent.K2_SetText` (`self.CountW3`) (`KismetTextLibrary.Conv_StringToText` (`KismetStringLibrary.Concat_StrStr` (`KismetStringLibrary.Conv_IntToString` (`KismetMathLibrary.Clamp` (+ (`KismetStringLibrary.Conv_StringToInt` (`KismetStringLibrary.Split` (`KismetTextLibrary.Conv_TextToString` (`TextRenderComponent.Text` (`self.CountW3`))) "/")) 1) 0 _goalcount)) "/" (`KismetStringLibrary.Conv_IntToString` _goalcount)))))

(fn `UserConstructionScript`)