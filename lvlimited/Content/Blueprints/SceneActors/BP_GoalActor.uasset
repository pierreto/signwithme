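; BP_GoalActor is a scene actor that displays collection progress for five letters (A, B, C, L, V) as "count/GoalCount" text.
; UpdateLetterCount maps a letter's sign to its text component, parses the current count from that text, increments it and clamps it to GoalCount.
; GetLetterTransform returns the world transform of the matching letter component.
; ResetLetterCount zeroes all counters, and Hide turns off visibility for the whole actor.
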(fn `GetLetterTransform`
  (params (Letter :type "/Game/Blueprints/SceneActors/BP_SignBlock Object Reference"))
  (returns (Location :type "Transform Structure"))
  (locals (LetterLocation :type "Transform Structure"))
  (switch `/Game/Blueprints/SceneActors/E_Signs` (`/Game/Blueprints/SceneActors/BP_SignBlock.Sign` Letter)
    (:`NewEnumerator1`
      (set `local.LetterLocation` (`SceneComponent.K2_GetComponentToWorld` (`self.FirstLetter`))))
    (:`NewEnumerator3`
      (set `local.LetterLocation` (`SceneComponent.K2_GetComponentToWorld` (`self.SecondLetter`))))
    (:`NewEnumerator4`
      (set `local.LetterLocation` (`SceneComponent.K2_GetComponentToWorld` (`self.ThirdLetter`))))
    (:`NewEnumerator0`
      (set `local.LetterLocation` (`SceneComponent.K2_GetComponentToWorld` (`self.FourthLetter`))))
    (:`NewEnumerator2`
      (set `local.LetterLocation` (`SceneComponent.K2_GetComponentToWorld` (`self.FifthLetter`)))))
  (return (`local.LetterLocation`)))

(fn `Hide`
  (`SceneComponent.SetVisibility` (`self.DefaultSceneRoot`) false true))

(fn `ResetLetterCount`
  (bind _returnvalue (`KismetTextLibrary.Conv_StringToText` (`KismetStringLibrary.Concat_StrStr` "0" "/" (`KismetStringLibrary.Conv_IntToString` (`self.GoalCount`)))))
  (`TextRenderComponent.K2_SetText` (`self.CountFirstLetter`) _returnvalue)
  (`TextRenderComponent.K2_SetText` (`self.CountSecondLetter`) _returnvalue)
  (`TextRenderComponent.K2_SetText` (`self.CountThirdLetter`) _returnvalue)
  (`TextRenderComponent.K2_SetText` (`self.CountFourthLetter`) _returnvalue)
  (`TextRenderComponent.K2_SetText` (`self.CountFifthLetter`) _returnvalue))

(fn `UpdateLetterCount`
  (params (Letter :type "/Game/Blueprints/SceneActors/BP_SignBlock Object Reference"))
  (locals (LetterToUpdate :type "TextRenderComponent Object Reference"))
  (bind _goalcount (`self.GoalCount`))
  (switch `/Game/Blueprints/SceneActors/E_Signs` (`/Game/Blueprints/SceneActors/BP_SignBlock.Sign` Letter)
    (:`NewEnumerator1`
      (set `local.LetterToUpdate` (`self.CountFirstLetter`)))
    (:`NewEnumerator3`
      (set `local.LetterToUpdate` (`self.CountSecondLetter`)))
    (:`NewEnumerator4`
      (set `local.LetterToUpdate` (`self.CountThirdLetter`)))
    (:`NewEnumerator0`
      (set `local.LetterToUpdate` (`self.CountFourthLetter`)))
    (:`NewEnumerator2`
      (set `local.LetterToUpdate` (`self.CountFifthLetter`))))
  (`TextRenderComponent.K2_SetText` (`local.LetterToUpdate`) (`KismetTextLibrary.Conv_StringToText` (`KismetStringLibrary.Concat_StrStr` (`KismetStringLibrary.Conv_IntToString` (`KismetMathLibrary.Clamp` (+ (`KismetStringLibrary.Conv_StringToInt` (`KismetStringLibrary.Split` (`KismetTextLibrary.Conv_TextToString` (`TextRenderComponent.Text` (`local.LetterToUpdate`))) "/")) 1) 0 _goalcount)) "/" (`KismetStringLibrary.Conv_IntToString` _goalcount)))))

(fn `UserConstructionScript`)