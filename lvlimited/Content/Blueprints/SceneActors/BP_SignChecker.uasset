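; BP_SignChecker is a scene actor that checks the player's current hand sign against the sign blocks from its Spawner.
; On BeginPlay it caches the player pawn as BP_Hands.
; Each Tick it compares the pawn's CurrentLetter with the enum name of the first initialized block in the Spawner's CurrentSignBlocks.
; On a match it tells the Spawner to destroy the current sign.
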(event `self.ReceiveBeginPlay`
  (bind _asbp_hands (cast `/Game/Blueprints/Characters/BP_Hands` (`GameplayStatics.GetPlayerPawn` 0)))
  (set `self.Player` _asbp_hands))

(event `self.ReceiveTick`
  (params (DeltaSeconds :type "Float (single-precision)"))
  (bind _player (`self.Player`))
  (if (`KismetSystemLibrary.IsValid` _player)
    (if (`self.CheckSign` (`/Game/Blueprints/Characters/BP_Hands.CurrentLetter` _player))
      (`/Game/Blueprints/SceneActors/BP_Spawner.DestroyCurrentSign` (`self.Spawner`)))))

(fn `CheckSign`
  (params (Sign :type String))
  (returns (Valid :type Boolean))
  (locals (Result :type Boolean))
  (bind _currentsignblocks (`/Game/Blueprints/SceneActors/BP_Spawner.CurrentSignBlocks` (`self.Spawner`)))
  (if (and (> (`KismetArrayLibrary.Array_Length` _currentsignblocks) 0) (`/Game/Blueprints/SceneActors/BP_SignBlock.Initialized` (`|GetArrayItem` _currentsignblocks)))
    (set `local.Result` (`KismetStringLibrary.EqualEqual_StrStr` (`|GetEnumeratorNameAsString` (`/Game/Blueprints/SceneActors/BP_SignBlock.Sign` (`|GetArrayItem` _currentsignblocks))) Sign))
    (else
      (set `local.Result` false)))
  (return (`local.Result`)))

(fn `UserConstructionScript`)