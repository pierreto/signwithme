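; Tutorial spawner that emits BP_SignBlock actors on a timer during Levels 1 and 2.
; A shuffled queue holds Number copies of each sign enum entry, and Tick spawns and tracks one block per interval.
; Level 2 start sets two copies per sign, resets the goal count to two, refills the queue and hides block replayers.
; MissCurrentSign requeues the first sign from BP_Spawner's list; DestroyCurrentSign's level-end call is unreachable.
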(event `self.ReceiveBeginPlay`
  (cast `/Game/Blueprints/Gameplay/BP_GameModeTuto` _)
  (set `self.GameStateRef` null)
  (bind _asbp_game_mode (cast `/Game/Blueprints/Gameplay/BP_GameMode` (`GameplayStatics.GetGameMode`)))
  (add `/Game/Blueprints/Gameplay/BP_GameMode.LevelStarted` _asbp_game_mode (delegate `LevelStarted`))
  (set `self.CurrentTimer` (`self.SpawnSpeed`) :!label _label)
  (`KismetArrayLibrary.Array_Clear` (`self.CurrentSignBlocks`))
  (for _index (range (enumcount `/Game/Blueprints/SceneActors/E_Signs`))
    (for _ (range (`self.Number`))
      (`KismetArrayLibrary.Array_Add` (`self.AvailableSigns`) (`KismetMathLibrary.Conv_IntToByte` _index))))
  (`KismetArrayLibrary.Array_Shuffle` (`self.AvailableSigns`)))

(event `LevelStarted`
  (params (Level :type Integer))
  (bind _output_get (set `self.HideHands` (== Level 2)))
  (if _output_get
    (set `self.Number` 2)
    (bind _outactors (`GameplayStatics.GetAllActorsOfClass` "/Game/Blueprints/SceneActors/BP_GoalActor.BP_GoalActor_C"))
    (bind _output (`|GetArrayItem` _outactors))
    (set `/Game/Blueprints/SceneActors/BP_GoalActor.GoalCount` 2 _output)
    (`/Game/Blueprints/SceneActors/BP_GoalActor.ResetLetterCount` _output)
    (goto _label)))

(event `self.ReceiveTick`
  (params (DeltaSeconds :type "Float (single-precision)"))
  (bind _availablesigns (`self.AvailableSigns`))
  (switch `/Game/Blueprints/Gameplay/GameStates` (`/Game/Blueprints/Gameplay/BP_GameState.GameState` (`.GameStateRef` (`self.GameStateRef`)))
    (:`NewEnumerator2`
      _)
    (:`NewEnumerator4`
      _))
  (bind _output_get (set `self.CurrentTimer` (- (`self.CurrentTimer`) DeltaSeconds)))
  (if (and (<= _output_get 0.0) (> (`KismetArrayLibrary.Array_Length` (`self.AvailableSigns`)) 0))
    (bind _returnvalue (`|SpawnActorFromClass` "/Game/Blueprints/SceneActors/BP_SignBlock.BP_SignBlock_C" (`self.GetTransform` self) "Undefined" "OverrideRootScale" null null))
    (set `/Game/Blueprints/SceneActors/BP_SignBlock.Sign` (cast `/Game/Blueprints/SceneActors/E_Signs` (`|GetArrayItem` _availablesigns)) _returnvalue)
    (`KismetArrayLibrary.Array_Remove` _availablesigns)
    (`/Game/Blueprints/SceneActors/BP_SignBlock.SetSignText` _returnvalue)
    (set `self.CurrentTimer` (`self.SpawnSpeed`))
    (`KismetArrayLibrary.Array_Add` (`self.CurrentSignBlocks`) _returnvalue)
    (`SceneComponent.SetVisibility` (`/Game/Blueprints/SceneActors/BP_SignBlock.Replayer` _returnvalue) (not (`self.HideHands`)) false)))

(fn `DestroyCurrentSign`
  (cast `/Game/Blueprints/Gameplay/BP_GameModeTuto` (`GameplayStatics.GetGameMode`)))

(fn `MissCurrentSign`
  (locals (CurrentSign :type "/Game/Blueprints/SceneActors/E_Signs Enum" :default "NewEnumerator1"))
  (bind _outactors (`GameplayStatics.GetAllActorsOfClass` "/Game/Blueprints/SceneActors/BP_Spawner.BP_Spawner_C"))
  (bind _currentsignblocks (`/Game/Blueprints/SceneActors/BP_Spawner.CurrentSignBlocks` (`|GetArrayItem` _outactors)))
  (set `local.CurrentSign` (`/Game/Blueprints/SceneActors/BP_SignBlock.Sign` (`|GetArrayItem` _currentsignblocks)))
  (`KismetArrayLibrary.Array_Remove` _currentsignblocks)
  (`KismetArrayLibrary.Array_Add` (`self.AvailableSigns`) (`local.CurrentSign`)))

(fn `UserConstructionScript`)