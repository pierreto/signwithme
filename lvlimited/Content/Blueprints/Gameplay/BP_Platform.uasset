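; BP_Platform is a gameplay platform whose mesh is tinted green or purple from a replicated Color variable.
; The Color RepNotify snaps the value to one of the two colors by testing its green channel.
; It then creates dynamic material instances for the platform and crest slots and sets their Color parameter.
; The event graph and construction script contain no logic.
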(fn `OnRep_Color`
  (locals (AssignedColor :type "LinearColor Structure"))
  (`|ExecutionSequence`
    (:`then_0`
      (if (>= (`.G` (`KismetMathLibrary.BreakColor` (`self.Color`))) 0.9)
        (set `local.AssignedColor` (`self.Green`))
        (else
          (set `local.AssignedColor` (`self.Purple`)))))
    (:`then_1`
      (bind _returnvalue (`PrimitiveComponent.CreateDynamicMaterialInstance` (`self.StaticMesh`) 0 "/Game/Assets/Material/Platform_Material.Platform_Material" "None"))
      (`MaterialInstanceDynamic.SetVectorParameterValue` _returnvalue "Color" (`local.AssignedColor`))
      (bind _returnvalue_2 (`PrimitiveComponent.CreateDynamicMaterialInstance` (`self.StaticMesh`) 1 "/Game/Assets/Material/Platform_Crest_Mat.Platform_Crest_Mat" "None"))
      (`MaterialInstanceDynamic.SetVectorParameterValue` _returnvalue_2 "Color" (`local.AssignedColor`)))))

(fn `UserConstructionScript`)