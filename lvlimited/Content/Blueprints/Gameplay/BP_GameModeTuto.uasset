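; Tutorial game mode that steps the player through letters A, B, C, L and V, then loads GameplayGym.
; Each OnLetterFinished advances the Tuto enum, greens the matching tagged sign block and, until V, timeline-rotates the tutorial spawner 60 degrees.
; Helper functions update score and combo on the player state and score actor, forward goal letters, swap tagged neon and level-change materials, and advance GameState levels.
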(event `self.ReceiveBeginPlay`
  (bind _asbp_player_state (cast `/Game/Blueprints/Gameplay/BP_PlayerState` (`Controller.PlayerState` (`GameplayStatics.GetPlayerController` 0))))
  (set `self.PlayerStateRef` _asbp_player_state)
  (set `/Game/Blueprints/Gameplay/BP_PlayerState.CurrentScore` 0.0 _asbp_player_state)
  (set `/Game/Blueprints/Gameplay/BP_PlayerState.CurrentMultiplier` 0.0 _asbp_player_state)
  (bind _asbp_game_state (cast `/Game/Blueprints/Gameplay/BP_GameState` (`GameplayStatics.GetGameState`)))
  (set `self.GameStateRef` _asbp_game_state)
  (set `self.Tuto` "NewEnumerator0"))

(event `self.ReceiveTick`
  (params (DeltaSeconds :type "Float (single-precision)"))
  (switch `/Game/Blueprints/Gameplay/TutorialStates` (`self.Tuto`)))

(event `OnLetterFinished`
  (switch `/Game/Blueprints/Gameplay/TutorialStates` (`self.Tuto`)
    (:`NewEnumerator0`
      (set `self.Tuto` "NewEnumerator1")
      (bind _outactors (`GameplayStatics.GetAllActorsOfClass` "/Game/Blueprints/SceneActors/BP_SignBlockLevel0.BP_SignBlockLevel0_C"))
      (for _array_element _outactors
        (if (`KismetArrayLibrary.Array_Contains` (`Actor.Tags` _array_element) "A")
          (`/Game/Blueprints/SceneActors/BP_SignBlockLevel0.GreenMeMommy` _array_element)
          (bind _outactors_2 (`GameplayStatics.GetAllActorsOfClass` "/Game/Blueprints/SceneActors/BP_TUTOSPAWN.BP_TUTOSPAWN_C"))
          (bind _output (`|GetArrayItem` _outactors_2))
          (bind _output_get (set `self.TargetRotation` (`KismetMathLibrary.MakeRotator` (.roll (`self.K2_GetActorRotation` _output)) (.pitch (`self.K2_GetActorRotation` _output)) (- (.yaw (`self.K2_GetActorRotation` _output)) 60.0))))
          (bind (_direction _newtrack_0) (`Timeline|Timeline_0`)
            (:`Update`
              (`self.K2_SetActorRotation` _output (`KismetMathLibrary.RLerp` (`self.K2_GetActorRotation` _output) _output_get _newtrack_0) false))))))
    (:`NewEnumerator1`
      (set `self.Tuto` "NewEnumerator2")
      (bind _outactors_3 (`GameplayStatics.GetAllActorsOfClass` "/Game/Blueprints/SceneActors/BP_SignBlockLevel0.BP_SignBlockLevel0_C"))
      (for _array_element_2 _outactors_3
        (if (`KismetArrayLibrary.Array_Contains` (`Actor.Tags` _array_element_2) "B")
          (`/Game/Blueprints/SceneActors/BP_SignBlockLevel0.GreenMeMommy` _array_element_2)
          (bind _outactors_4 (`GameplayStatics.GetAllActorsOfClass` "/Game/Blueprints/SceneActors/BP_TUTOSPAWN.BP_TUTOSPAWN_C"))
          (bind _output_2 (`|GetArrayItem` _outactors_4))
          (bind _output_get_2 (set `self.TargetRotation` (`KismetMathLibrary.MakeRotator` (.roll (`self.K2_GetActorRotation` _output_2)) (.pitch (`self.K2_GetActorRotation` _output_2)) (- (.yaw (`self.K2_GetActorRotation` _output_2)) 60.0))))
          (bind (_direction_2 _newtrack_0_2) (`Timeline|Timeline_1`)
            (:`Update`
              (`self.K2_SetActorRotation` _output_2 (`KismetMathLibrary.RLerp` (`self.K2_GetActorRotation` _output_2) _output_get_2 _newtrack_0_2) false))))))
    (:`NewEnumerator2`
      (set `self.Tuto` "NewEnumerator3")
      (bind _outactors_5 (`GameplayStatics.GetAllActorsOfClass` "/Game/Blueprints/SceneActors/BP_SignBlockLevel0.BP_SignBlockLevel0_C"))
      (for _array_element_3 _outactors_5
        (if (`KismetArrayLibrary.Array_Contains` (`Actor.Tags` _array_element_3) "C")
          (`/Game/Blueprints/SceneActors/BP_SignBlockLevel0.GreenMeMommy` _array_element_3)
          (bind _outactors_6 (`GameplayStatics.GetAllActorsOfClass` "/Game/Blueprints/SceneActors/BP_TUTOSPAWN.BP_TUTOSPAWN_C"))
          (bind _output_3 (`|GetArrayItem` _outactors_6))
          (bind _output_get_3 (set `self.TargetRotation` (`KismetMathLibrary.MakeRotator` (.roll (`self.K2_GetActorRotation` _output_3)) (.pitch (`self.K2_GetActorRotation` _output_3)) (- (.yaw (`self.K2_GetActorRotation` _output_3)) 60.0))))
          (bind (_direction_3 _newtrack_0_3) (`Timeline|Timeline_2`)
            (:`Update`
              (`self.K2_SetActorRotation` _output_3 (`KismetMathLibrary.RLerp` (`self.K2_GetActorRotation` _output_3) _output_get_3 _newtrack_0_3) false))))))
    (:`NewEnumerator3`
      (set `self.Tuto` "NewEnumerator4")
      (bind _outactors_7 (`GameplayStatics.GetAllActorsOfClass` "/Game/Blueprints/SceneActors/BP_SignBlockLevel0.BP_SignBlockLevel0_C"))
      (for _array_element_4 _outactors_7
        (if (`KismetArrayLibrary.Array_Contains` (`Actor.Tags` _array_element_4) "L")
          (`/Game/Blueprints/SceneActors/BP_SignBlockLevel0.GreenMeMommy` _array_element_4)
          (bind _outactors_8 (`GameplayStatics.GetAllActorsOfClass` "/Game/Blueprints/SceneActors/BP_TUTOSPAWN.BP_TUTOSPAWN_C"))
          (bind _output_4 (`|GetArrayItem` _outactors_8))
          (bind _output_get_4 (set `self.TargetRotation` (`KismetMathLibrary.MakeRotator` (.roll (`self.K2_GetActorRotation` _output_4)) (.pitch (`self.K2_GetActorRotation` _output_4)) (- (.yaw (`self.K2_GetActorRotation` _output_4)) 60.0))))
          (bind (_direction_4 _newtrack_0_4) (`Timeline|Timeline_3`)
            (:`Update`
              (`self.K2_SetActorRotation` _output_4 (`KismetMathLibrary.RLerp` (`self.K2_GetActorRotation` _output_4) _output_get_4 _newtrack_0_4) false))))))
    (:`NewEnumerator4`
      (bind _outactors_9 (`GameplayStatics.GetAllActorsOfClass` "/Game/Blueprints/SceneActors/BP_SignBlockLevel0.BP_SignBlockLevel0_C"))
      (for _array_element_5 _outactors_9
        (if (`KismetArrayLibrary.Array_Contains` (`Actor.Tags` _array_element_5) "v")
          (`/Game/Blueprints/SceneActors/BP_SignBlockLevel0.GreenMeMommy` _array_element_5)
          (`KismetSystemLibrary.Delay` 5.0)
          (`GameplayStatics.OpenLevel` "GameplayGym"))))))

(fn `AddCombo`
  (bind _playerstateref (`self.PlayerStateRef`))
  (set `/Game/Blueprints/Gameplay/BP_PlayerState.CurrentMultiplier` (+ (`/Game/Blueprints/Gameplay/BP_PlayerState.CurrentMultiplier` _playerstateref) 1.0) _playerstateref)
  (bind _outactors (`GameplayStatics.GetAllActorsOfClass` "/Game/Blueprints/SceneActors/BP_ScoreActor.BP_ScoreActor_C"))
  (bind _output_get (set `self.Score` (`|GetArrayItem` _outactors)))
  (`/Game/Blueprints/SceneActors/BP_ScoreActor.SetMultiplierText` _output_get (`KismetMathLibrary.FTrunc` (`/Game/Blueprints/Gameplay/BP_PlayerState.CurrentMultiplier` (`self.PlayerStateRef`)))))

(fn `AddScore`
  (bind _playerstateref (`self.PlayerStateRef`))
  (set `/Game/Blueprints/Gameplay/BP_PlayerState.CurrentScore` (+ (`/Game/Blueprints/Gameplay/BP_PlayerState.CurrentScore` _playerstateref) 1.0) _playerstateref)
  (bind _outactors (`GameplayStatics.GetAllActorsOfClass` "/Game/Blueprints/SceneActors/BP_ScoreActor.BP_ScoreActor_C"))
  (bind _output_get (set `self.Score` (`|GetArrayItem` _outactors)))
  (`/Game/Blueprints/SceneActors/BP_ScoreActor.SetScoreText` _output_get (`/Game/Blueprints/Gameplay/BP_PlayerState.CurrentScore` (`self.PlayerStateRef`))))

(fn `AssignBlackLevelChange`
  (bind _outactors (`GameplayStatics.GetAllActorsWithTag` "LevelChange"))
  (for _array_element _outactors
    (`PrimitiveComponent.CreateDynamicMaterialInstance` (`self.GetComponentByClass` _array_element "/Script/Engine.MeshComponent") 0 "/Game/Assets/Material/EBase.EBase" "None")))

(fn `AssignBlueNeon`
  (bind _outactors (`GameplayStatics.GetAllActorsWithTag` "Neon"))
  (for _array_element _outactors
    (`PrimitiveComponent.CreateDynamicMaterialInstance` (`self.GetComponentByClass` _array_element "/Script/Engine.MeshComponent") 0 "/Game/Assets/Material/EBlue.EBlue" "None")))

(fn `AssignRedNeon`
  (bind _outactors (`GameplayStatics.GetAllActorsWithTag` "Neon"))
  (for _array_element _outactors
    (`PrimitiveComponent.CreateDynamicMaterialInstance` (`self.GetComponentByClass` _array_element "/Script/Engine.MeshComponent") 0 "/Game/Assets/Material/ERed.ERed" "None")))

(fn `AssignWhiteLevelChange`
  (bind _outactors (`GameplayStatics.GetAllActorsWithTag` "LevelChange"))
  (for _array_element _outactors
    (`PrimitiveComponent.CreateDynamicMaterialInstance` (`self.GetComponentByClass` _array_element "/Script/Engine.MeshComponent") 0 "/Game/Assets/Material/EWhite.EWhite" "None")))

(fn `LevelEnded`
  (switch `/Game/Blueprints/Gameplay/GameStates` (`/Game/Blueprints/Gameplay/BP_GameState.GameState` (`self.GameStateRef`))
    (:`NewEnumerator2`
      (set `/Game/Blueprints/Gameplay/BP_GameState.GameState` "NewEnumerator4" (`self.GameStateRef`)))
    (:`NewEnumerator4`
      (bind _outactors (`GameplayStatics.GetAllActorsOfClass` "/Game/Blueprints/SceneActors/BP_GoalThirdLevelActor.BP_GoalThirdLevelActor_C"))
      (`/Game/Blueprints/SceneActors/BP_GoalThirdLevelActor.Show` (`|GetArrayItem` _outactors))
      (bind _outactors_2 (`GameplayStatics.GetAllActorsOfClass` "/Game/Blueprints/SceneActors/BP_GoalActor.BP_GoalActor_C"))
      (`/Game/Blueprints/SceneActors/BP_GoalActor.Hide` (`|GetArrayItem` _outactors_2))
      (set `/Game/Blueprints/Gameplay/BP_GameState.GameState` "NewEnumerator5" (`self.GameStateRef`)))
    (:`NewEnumerator5`
      (set `/Game/Blueprints/Gameplay/BP_GameState.GameState` "NewEnumerator3" (`self.GameStateRef`)))))

(fn `ResetCombo`
  (set `/Game/Blueprints/Gameplay/BP_PlayerState.CurrentMultiplier` 0.0 (`self.PlayerStateRef`))
  (bind _outactors (`GameplayStatics.GetAllActorsOfClass` "/Game/Blueprints/SceneActors/BP_ScoreActor.BP_ScoreActor_C"))
  (bind _output_get (set `self.Score` (`|GetArrayItem` _outactors)))
  (`/Game/Blueprints/SceneActors/BP_ScoreActor.SetMultiplierText` _output_get (`KismetMathLibrary.FTrunc` (`/Game/Blueprints/Gameplay/BP_PlayerState.CurrentMultiplier` (`self.PlayerStateRef`)))))

(fn `UpdateGoal`
  (params (Letter :type "/Game/Blueprints/SceneActors/BP_SignBlock Object Reference"))
  (bind _outactors (`GameplayStatics.GetAllActorsOfClass` "/Game/Blueprints/SceneActors/BP_GoalActor.BP_GoalActor_C"))
  (`/Game/Blueprints/SceneActors/BP_GoalActor.UpdateLetterCount` (`|GetArrayItem` _outactors) Letter))

(fn `UserConstructionScript`)