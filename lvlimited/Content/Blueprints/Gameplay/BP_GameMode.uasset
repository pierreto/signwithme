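; Game mode that runs a three-level progression with score, combo multiplier and letter goal tracking.
; BeginPlay resets player state and sets Level1; Tick fires a one-shot LevelStarted call per level, and LevelEnded advances the game state.
; Score and combo functions update player state and the first BP_ScoreActor's text, while UpdateGoal forwards letters to BP_GoalActor.
; OnMiss flashes Neon-tagged meshes red and blue by swapping materials.
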(event `self.ReceiveBeginPlay`
  (bind _playerstateref (`self.PlayerStateRef`))
  (bind _asbp_player_state (cast `/Game/Blueprints/Gameplay/BP_PlayerState` (`Controller.PlayerState` (`GameplayStatics.GetPlayerController` 0))))
  (set `self.PlayerStateRef` _asbp_player_state)
  (set `/Game/Blueprints/Gameplay/BP_PlayerState.CurrentScore` 0.0 _asbp_player_state)
  (set `/Game/Blueprints/Gameplay/BP_PlayerState.CurrentMultiplier` 0.0 _asbp_player_state)
  (bind _asbp_game_state (cast `/Game/Blueprints/Gameplay/BP_GameState` (`GameplayStatics.GetGameState`)))
  (set `self.GameStateRef` _asbp_game_state)
  (bind _outactors (`GameplayStatics.GetAllActorsOfClass` "/Script/Engine.PlayerStart"))
  (bind _outactors_2 (`GameplayStatics.GetAllActorsOfClass` "/Game/Blueprints/SceneActors/BP_ScoreActor.BP_ScoreActor_C"))
  (bind _output_get (set `self.Score` (`|GetArrayItem` _outactors_2)))
  (`/Game/Blueprints/SceneActors/BP_ScoreActor.SetScoreText` _output_get (`/Game/Blueprints/Gameplay/BP_PlayerState.CurrentScore` _playerstateref))
  ;[1 1 1] Straight start
  (`/Game/Blueprints/SceneActors/BP_ScoreActor.SetMultiplierText` _output_get (`KismetMathLibrary.FTrunc` (`/Game/Blueprints/Gameplay/BP_PlayerState.CurrentMultiplier` _playerstateref)))
  (set `/Game/Blueprints/Gameplay/BP_GameState.GameState` "NewEnumerator2" (`self.GameStateRef`)))

(event `self.ReceiveTick`
  (params (DeltaSeconds :type "Float (single-precision)"))
  (switch `/Game/Blueprints/Gameplay/GameStates` (`/Game/Blueprints/Gameplay/BP_GameState.GameState` (`self.GameStateRef`))
    (:`NewEnumerator2`
      (`/Engine/EditorBlueprintResources/StandardMacros.DoOnce` false
        (:`Completed`
          (`self.LevelStarted` 1))))
    (:`NewEnumerator4`
      (`/Engine/EditorBlueprintResources/StandardMacros.DoOnce` false
        (:`Completed`
          (`self.LevelStarted` 2))))
    (:`NewEnumerator5`
      (`/Engine/EditorBlueprintResources/StandardMacros.DoOnce` false
        (:`Completed`
          (`self.LevelStarted` 3))))))

(event `OnMiss`
  (`self.AssignRedNeon`)
  (`KismetSystemLibrary.Delay` 0.2)
  (`self.AssignBlueNeon`)
  (`KismetSystemLibrary.Delay` 0.2)
  (`self.AssignRedNeon`)
  (`KismetSystemLibrary.Delay` 0.2)
  (`self.AssignBlueNeon`))

(event `OnRedTriggered`)

(fn `AddCombo`
  (bind _playerstateref (`self.PlayerStateRef`))
  (set `/Game/Blueprints/Gameplay/BP_PlayerState.CurrentMultiplier` (+ (`/Game/Blueprints/Gameplay/BP_PlayerState.CurrentMultiplier` _playerstateref) 1.0) _playerstateref)
  (bind _outactors (`GameplayStatics.GetAllActorsOfClass` "/Game/Blueprints/SceneActors/BP_ScoreActor.BP_ScoreActor_C"))
  (bind _output_get (set `self.Score` (`|GetArrayItem` _outactors)))
  (`/Game/Blueprints/SceneActors/BP_ScoreActor.SetMultiplierText` _output_get (`KismetMathLibrary.FTrunc` (`/Game/Blueprints/Gameplay/BP_PlayerState.CurrentMultiplier` (`self.PlayerStateRef`)))))

(fn `AddScore`
  (bind _playerstateref (`self.PlayerStateRef`))
  (set `/Game/Blueprints/Gameplay/BP_PlayerState.CurrentScore` (+ (`/Game/Blueprints/Gameplay/BP_PlayerState.CurrentScore` _playerstateref) 1.0) _playerstateref)
  (bind _outactors (`GameplayStatics.GetAllActorsOfClass` "/Game/Blueprints/SceneActors/BP_ScoreActor.BP_ScoreActor_C"))
  (bind _output_get (set `self.Score` (`|GetArrayItem` _outactors)))
  (`/Game/Blueprints/SceneActors/BP_ScoreActor.SetScoreText` _output_get (`/Game/Blueprints/Gameplay/BP_PlayerState.CurrentScore` (`self.PlayerStateRef`))))

(fn `AssignBlueNeon`
  (bind _outactors (`GameplayStatics.GetAllActorsWithTag` "Neon"))
  (for _array_element _outactors
    (`PrimitiveComponent.CreateDynamicMaterialInstance` (`self.GetComponentByClass` _array_element "/Script/Engine.MeshComponent") 0 "/Game/Assets/Material/EBlue.EBlue" "None")))

(fn `AssignRedNeon`
  (bind _outactors (`GameplayStatics.GetAllActorsWithTag` "Neon"))
  (for _array_element _outactors
    (`PrimitiveComponent.CreateDynamicMaterialInstance` (`self.GetComponentByClass` _array_element "/Script/Engine.MeshComponent") 0 "/Game/Assets/Material/ERed.ERed" "None")))

(fn `LevelEnded`
  (switch `/Game/Blueprints/Gameplay/GameStates` (`/Game/Blueprints/Gameplay/BP_GameState.GameState` (`self.GameStateRef`))
    (:`NewEnumerator2`
      (set `/Game/Blueprints/Gameplay/BP_GameState.GameState` "NewEnumerator4" (`self.GameStateRef`)))
    (:`NewEnumerator4`
      (set `/Game/Blueprints/Gameplay/BP_GameState.GameState` "NewEnumerator5" (`self.GameStateRef`)))
    (:`NewEnumerator5`
      (set `/Game/Blueprints/Gameplay/BP_GameState.GameState` "NewEnumerator3" (`self.GameStateRef`)))))

(fn `ResetCombo`
  (set `/Game/Blueprints/Gameplay/BP_PlayerState.CurrentMultiplier` 0.0 (`self.PlayerStateRef`))
  (bind _outactors (`GameplayStatics.GetAllActorsOfClass` "/Game/Blueprints/SceneActors/BP_ScoreActor.BP_ScoreActor_C"))
  (bind _output_get (set `self.Score` (`|GetArrayItem` _outactors)))
  (`/Game/Blueprints/SceneActors/BP_ScoreActor.SetMultiplierText` _output_get (`KismetMathLibrary.FTrunc` (`/Game/Blueprints/Gameplay/BP_PlayerState.CurrentMultiplier` (`self.PlayerStateRef`)))))

(fn `UpdateGoal`
  (params (Letter :type "/Game/Blueprints/SceneActors/BP_SignBlock Object Reference"))
  (bind _outactors (`GameplayStatics.GetAllActorsOfClass` "/Game/Blueprints/SceneActors/BP_GoalActor.BP_GoalActor_C"))
  (`/Game/Blueprints/SceneActors/BP_GoalActor.UpdateLetterCount` (`|GetArrayItem` _outactors) Letter))

(fn `UserConstructionScript`)